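; Projectile actor that flies along world X, destroys BP_Obstacle actors it hits and awards score to its owning player.
; Tick moves it with a swept world offset and destroys it after a few seconds; SetPlayerSpeed adds the passed speed to its launch speed.
; Cylinder overlaps handle obstacle hits, and also destroy the projectile when the other component's collision is query-only or physics-only.
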(event `self.ReceiveTick`
  (params (DeltaSeconds :type "Float (single-precision)"))
  (`|ExecutionSequence`
    (:`then_0`
      (`self.K2_AddActorWorldOffset` (`KismetMathLibrary.MakeVector` (* DeltaSeconds (`self.ForwardSpeed`))) true))
    (:`then_1`
      (bind _output_get (set `self.Age` (+ DeltaSeconds (`self.Age`))))
      (`/Engine/EditorBlueprintResources/StandardMacros.CompareFloat` _output_get 6.0
        (:`>`
          (`self.K2_DestroyActor`))))))

(event `self.Cylinder.OnComponentBeginOverlap`
  (params (OverlappedComponent :type "PrimitiveComponent Object Reference") (OtherActor :type "Actor Object Reference") (OtherComp :type "PrimitiveComponent Object Reference") (OtherBodyIndex :type Integer) (bFromSweep :type Boolean) (SweepResult :type "HitResult Structure (by ref)"))
  (`|ExecutionSequence`
    (:`then_0`
      (bind _asbp_obstacle (cast `/Game/InfiniteMatrix/Blueprints/BP_Obstacle` OtherActor))
      (`/Game/InfiniteMatrix/Blueprints/BP_Player.ChangeScore` (`self.PlayerOwner`) 2)
      (`self.K2_DestroyActor` _asbp_obstacle))
    (:`then_1`
      (switch `ECollisionEnabled` (`PrimitiveComponent.GetCollisionEnabled` OtherComp)
        (:`QueryOnly`
          _)
        (:`PhysicsOnly`
          _))
      (`self.K2_DestroyActor`))))

(fn `SetPlayerSpeed`
  (params (NewParam :type "Float (double-precision)"))
  (set `self.ForwardSpeed` (+ (`self.ForwardLaunch`) NewParam)))

(fn `UserConstructionScript`)